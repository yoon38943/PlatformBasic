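; General Blueprint function library that creates pop-up and loading screen widgets and surfaces stored network or travel errors.
; Widget helpers add WBP_PopUp or WBP_LoadingScreen to the viewport for player controller 0 if it is local.
; The error check reads BP_GI's error strings and shows an OK pop-up, prioritizing network errors.
; Both error branches clear only the travel error, leaving the network error set.
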(fn `CheckFor_ActiveError`
  (bind _active_error (`self.IsActiveError` null))
  (if _active_error
    (bind _asbp_gi (cast `/Game/Framework/BP_GI` (`GameplayStatics.GetGameInstance` null)))
    (bind _hnetworkerror (`PlatformGI.HNetworkError` _asbp_gi))
    (if (`KismetStringLibrary.IsEmpty` _hnetworkerror)
      (bind _htravelerror (`PlatformGI.HTravelError` _asbp_gi))
      (if (not (`KismetStringLibrary.IsEmpty` _htravelerror))
        (`self.CreateErrorPopup` _htravelerror)
        (set `PlatformGI.HTravelError` "" _asbp_gi))
      (else
        (`self.CreateErrorPopup` _hnetworkerror)
        (set `PlatformGI.HTravelError` "" _asbp_gi)))
    (return)))

(fn `Create_LoadingScreen`
  (bind _returnvalue (`GameplayStatics.GetPlayerController` null))
  (if (`Controller.IsLocalPlayerController` _returnvalue)
    (bind _returnvalue_2 (`|CreateWidget` "/Game/UI/WBP_LoadingScreen.WBP_LoadingScreen_C" _returnvalue))
    (`UserWidget.AddToViewport` _returnvalue_2 0)))

(fn `Create_PopUp`
  (params (PopUp_Message :type Text) (Left_Button_Text :type Text) (Show_Right_Button :type Boolean) (Right_Button_Text :type Text))
  (returns (ReturnValue :type "/Game/UI/WBP_PopUp Object Reference"))
  (bind _returnvalue (`GameplayStatics.GetPlayerController` null))
  (if (`Controller.IsLocalPlayerController` _returnvalue)
    (bind _returnvalue_2 (`|CreateWidget` "/Game/UI/WBP_PopUp.WBP_PopUp_C" _returnvalue PopUp_Message Left_Button_Text Show_Right_Button Right_Button_Text))
    (`UserWidget.AddToViewport` _returnvalue_2 0)
    (return _returnvalue_2)))

(fn `CreateErrorPopup`
  (params (`Error Message` :type String))
  (`self.Create_PopUp` (`KismetTextLibrary.Conv_StringToText` (`KismetStringLibrary.Concat_StrStr` "Error: " `Error Message`)) "OK")
  (return))

(fn `IsActiveError`
  (returns (`Active Error` :type Boolean))
  (bind _asbp_gi (cast `/Game/Framework/BP_GI` (`GameplayStatics.GetGameInstance` null)))
  (if (`KismetStringLibrary.IsEmpty` (`PlatformGI.HNetworkError` _asbp_gi))
    (if (`KismetStringLibrary.IsEmpty` (`PlatformGI.HTravelError` _asbp_gi))
      (return false)
      (else
        (return true)))
    (else
      (return true))))