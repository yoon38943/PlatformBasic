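; BP_PlatformGameState is the game state for a platform game's rounds, holding the start countdown and winner reference.
; On BeginPlay the server decrements RoundCountdown once after a one-second delay; no loop is shown.
; Helper functions play chimes, trigger the local controller's Ready-Go animation at count two, and enable character movement through BP_PlatformGameMode.
; The WinnerRef RepNotify marks the round ended on authority.
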(event `self.ReceiveBeginPlay`
  (`/Engine/EditorBlueprintResources/ActorMacros.Switch Has Authority`
    (:`Authority`
      (`self.Countdwon`))))

(event `Countdwon`
  (`KismetSystemLibrary.Delay` 1.0)
  (bind _result (`/Engine/EditorBlueprintResources/StandardMacros.DecrementInt` (`self.RoundCountdown`))
    (:`  `
      (set `self.RoundCountdown` _result))))

(fn `OnRep_WinnerRef`
  (`/Engine/EditorBlueprintResources/ActorMacros.Switch Has Authority`
    (:`Authority`
      (set `self.IsRoundEnded` true))))

(fn `PlayCountDownSound`
  (if (== (`self.RoundCountdown`) 0)
    (`GameplayStatics.PlaySound2D` "/Game/Audio/Cues/SC_Countdown_Chime_final.SC_Countdown_Chime_final" 1.0 1.0 0.0 null null)
    (else
      (`GameplayStatics.PlaySound2D` "/Game/Audio/Cues/SC_Countdown_chime.SC_Countdown_chime" 1.0 1.0 0.0 null null))))

(fn `PlayReadyGoAnimation`
  (if (== (`self.RoundCountdown`) 2)
    (bind _asbp_platform_player_controller (cast `/Game/Framework/BP_PlatformPlayerController` (`GameplayStatics.GetPlayerController` 0)))
    (`/Game/Framework/BP_PlatformPlayerController.OC_PlayReadyGoAnimation` _asbp_platform_player_controller)))

(fn `StartRound`
  ; 캐릭터를 움직이게 한다.( GameMode )
  (bind _asbp_platform_game_mode (cast `/Game/Framework/BP_PlatformGameMode` (`GameplayStatics.GetGameMode`)))
  (`/Game/Framework/BP_PlatformGameMode.EnableCharacterMovement` _asbp_platform_game_mode))

(fn `UserConstructionScript`)