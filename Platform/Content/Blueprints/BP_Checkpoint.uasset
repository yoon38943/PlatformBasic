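; BP_Checkpoint is a checkpoint actor that records a player's progress when their platform character enters its box trigger.
; On overlap, only the server casts to BP_PlatformCharacter and writes CheckPointID into the CheckPointTag of that character's PlatformPlayerState.
; The construction script sets a text render to "Check Point" plus the ID, labelling each placed instance.
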(event `self.Box.OnComponentBeginOverlap`
  (params (OverlappedComponent :type "PrimitiveComponent Object Reference") (OtherActor :type "Actor Object Reference") (OtherComp :type "PrimitiveComponent Object Reference") (OtherBodyIndex :type Integer) (bFromSweep :type Boolean) (SweepResult :type "HitResult Structure (by ref)"))
  (`/Engine/EditorBlueprintResources/ActorMacros.Switch Has Authority`
    (:`Authority`
      (bind _asbp_platform_character (cast `/Game/Character/BP_PlatformCharacter` OtherActor))
      (bind _asplatform_player_state (cast `PlatformPlayerState` (`Pawn.PlayerState` _asbp_platform_character)))
      (set `PlatformPlayerState.CheckPointTag` (`self.CheckPointID`) _asplatform_player_state))))

(fn `UserConstructionScript`
  (`TextRenderComponent.K2_SetText` (`self.TextRender`) (`KismetTextLibrary.Conv_StringToText` (`KismetStringLibrary.Concat_StrStr` "Check Point " (`KismetStringLibrary.Conv_NameToString` (`self.CheckPointID`))))))