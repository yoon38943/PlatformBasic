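; BP_Trophy is a pickup that decides the winner of a platformer match.
; On the server, the first mesh overlap passes a DoOnce before the character cast, then writes that BP_PlatformCharacter's PlayerState into BP_PlatformGameState's WinnerRef.
; MC_SpawnPoof then plays the poof effect and sound at the trophy, and only the authority destroys the actor.
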(event `self.StaticMesh.OnComponentBeginOverlap`
  (params (OverlappedComponent :type "PrimitiveComponent Object Reference") (OtherActor :type "Actor Object Reference") (OtherComp :type "PrimitiveComponent Object Reference") (OtherBodyIndex :type Integer) (bFromSweep :type Boolean) (SweepResult :type "HitResult Structure (by ref)"))
  (`/Engine/EditorBlueprintResources/ActorMacros.Switch Has Authority`
    (:`Authority`
      (`/Engine/EditorBlueprintResources/StandardMacros.DoOnce` false
        (:`Completed`
          (bind _asbp_platform_character (cast `/Game/Character/BP_PlatformCharacter` OtherActor))
          (bind _asbp_platform_game_state (cast `/Game/Framework/BP_PlatformGameState` (`GameplayStatics.GetGameState`)))
          (set `/Game/Framework/BP_PlatformGameState.WinnerRef` (`Pawn.PlayerState` _asbp_platform_character) _asbp_platform_game_state)
          (`self.MC_SpawnPoof`))))))

(event `MC_SpawnPoof`
  (`NiagaraFunctionLibrary.SpawnSystemAtLocation` "/Game/Niagara/NS_Poof.NS_Poof" (`self.K2_GetActorLocation`))
  (`GameplayStatics.PlaySoundAtLocation` "/Game/Audio/Cues/SC_Poof.SC_Poof" (`self.K2_GetActorLocation`) (struct) 1.0 1.0 0.0 null null null null)
  (`/Engine/EditorBlueprintResources/ActorMacros.Switch Has Authority`
    (:`Authority`
      (`self.K2_DestroyActor`))))

(fn `UserConstructionScript`)